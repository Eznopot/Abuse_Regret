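; Finish-line platform that records each player's placing when they overlap its Box trigger.
; A PlayerCharacter without a place takes the GameState's finished-player count, which then increments on every overlap, even repeat ones.
; Each overlap also decrements the GameState's max-player count; if the result equals that player's place, the GameInstance returns to the lobby after a short delay.
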(event OnComponentBeginOverlap(Box)
  (params (OverlappedComponent :type Primitive%20Component%20Object%20Reference) (OtherActor :type Actor%20Object%20Reference) (OtherComp :type Primitive%20Component%20Object%20Reference) (OtherBodyIndex :type Integer) (bFromSweep :type Boolean) (SweepResult :type Hit%20Result%20Structure%20%28by%20ref%29))
  (bind _returnvalue (Game|GetGameState))
  (bind _asplayer_character (Utilities|Casting|CastToPlayerCharacter OtherActor))
  (bind _asmy_game_state (Utilities|Casting|CastToMyGameState _returnvalue))
  (Utilities|FlowControl|Sequence
    (:then_0
      (if (== (Variables|/Game/Abuse_regret/Blueprints/PlayerCharacter.PlayerCharacter_C|GetMyPlace _asplayer_character) -1)
        (Variables|/Game/Abuse_regret/Blueprints/PlayerCharacter.PlayerCharacter_C|SetMyPlace _asplayer_character (stale _output_get))))
    (:then_1
      (bind _result (Math|Integer|IncrementInt (Variables|/Game/Abuse_regret/core/MyGameState.MyGameState_C|GetnbPlayerFinish _asmy_game_state))
        (:%20%20
          (bind _output_get (Variables|/Game/Abuse_regret/core/MyGameState.MyGameState_C|SetnbPlayerFinish _asmy_game_state _result)))))
    (:then_2
      (bind _result_2 (Math|Integer|DecrementInt (Variables|/Game/Abuse_regret/core/MyGameState.MyGameState_C|GetnbPlayerMax _asmy_game_state))
        (:%20%20
          (if (== _result_2 (Variables|/Game/Abuse_regret/Blueprints/PlayerCharacter.PlayerCharacter_C|GetMyPlace (.AsPlayer%20Character (Utilities|Casting|CastToPlayerCharacter OtherActor))))
            (Utilities|FlowControl|Delay 3.0)
            (Default|ReturntoLobby (.AsMy%20Game%20Instance (Utilities|Casting|CastToMyGameInstance (Game|GetGameInstance))))))))))

(fn ConstructionScript)